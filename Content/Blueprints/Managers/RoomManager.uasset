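; RoomManager drives procedural room streaming, loading randomly chosen exit levels ahead of the player and unloading the rooms left behind.
; When the player enters the trigger, it animates the door, unloads the other recorded rooms, then loads shuffled ExitLevels, one per exit anchor.
; Messages align each new room's entrance root to its anchor and pass along connected-room names.
; Manual counter loops sequence the latent load and unload calls.
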(event OnComponentBeginOverlap(EnteredTrigger)
  (params (OtherActor :type Actor%20Object%20Reference) (OtherComp :type Primitive%20Component%20Object%20Reference) (OtherBodyIndex :type Integer) (bFromSweep :type Boolean) (SweepResult :type Hit%20Result%20Structure%20%28by%20ref%29))
  ;[1 1 1] Did the player enter our Room Trigger?
  (if (Utilities|DoesObjectImplementInterface OtherActor "/Game/Blueprints/Interfaces/PlayerInterface.PlayerInterface_C") ; Is this the player?
    (Default|AnimateDoor (Variables|Default|GetDoorToClose)) ; Tell the door to animate
    (Utilities|FlowControl|Delay 2.0) ; Wait for the Animation to end
    ;;[0.2646 1 0.4485] Our fake loop since For Loop has issues with Unload Stream Level giving control back to the loop while it works
    (Variables|Default|SetUnloadingLevelsLoopCount 0) ; Start our loop from the start
    (if (Utilities|Name|NotEqual(Name) (Utilities|Array|Get(acopy) (Variables|Default|GetRoomsCameFrom) (Variables|Default|GetUnloadingLevelsLoopCount)) (Variables|Default|GetCurrentRoom)) :!label _label ; Is this the current room?
      (Game|UnloadStreamLevel(byName) (Utilities|Array|Get(acopy) (Variables|Default|GetRoomsCameFrom) (Variables|Default|GetUnloadingLevelsLoopCount))) ; Unload a previous room
    )
    (if (== (Variables|Default|GetUnloadingLevelsLoopCount) (- (Utilities|Array|Length (Variables|Default|GetRoomsCameFrom)) 1)) ; Have we unloaded all the previous rooms?
      (CallFunction|SpawnExitRooms) ; Spawn the new rooms connecting to this one
      (else
        (Variables|Default|SetUnloadingLevelsLoopCount (+ (Variables|Default|GetUnloadingLevelsLoopCount) 1)) ; Increment our loop and go to the next room
        (goto _label)))))

(event Custom|SpawnExitRooms
  (bind _spawnablerooms (Variables|Default|GetSpawnableRooms))
  ;[1 1 1] Spawn our Exit Rooms
  (if (not (Variables|Default|GetHasSpawnedExitRooms)) ; Have we spawned them already?
    (Utilities|Array|Clear (Variables|Default|GetConnectedRooms)) ; Clear our Connected Rooms Array
    (Utilities|Array|Clear _spawnablerooms) ; Clear our Spawned Rooms Array
    (Utilities|Array|AppendArray _spawnablerooms (Variables|Default|GetExitLevels)) ; Fill our Spawnable Rooms Array with the Valid Levels
    (Utilities|Array|Shuffle (Variables|Default|GetSpawnableRooms)) ; Randomize our available rooms
    (Game|LoadStreamLevel(byName) (CallFunction|WhichRoomtoSpawn) true :!label _label) ; Load up the random level
    (Class|RoomInterfaces|AlignEntracetoExit(Message) (Class|GameplayStatics|GetStreamingLevel (CallFunction|WhichRoomtoSpawn)) (Transformation|GetActorTransform (Utilities|Array|Get(acopy) (Variables|Default|GetExitAnchors) (Variables|Default|GetLoadingLevelsLoopCount)))) ; Align the entrance of the spawned level to the exit anchor
    (Utilities|Array|Add (Variables|Default|GetConnectedRooms) (CallFunction|WhichRoomtoSpawn)) ; Add this room name to the connected rooms array
    (if (== (Variables|Default|GetLoadingLevelsLoopCount) (- (Utilities|Array|Length (Variables|Default|GetExitAnchors)) 1)) ; Are we done spawning?
      (Variables|Default|SetHasSpawnedExitRooms true) ; Make sure we dont spawn rooms again
      (CallFunction|PassConnectedRoomstoNewRooms) ; Let the new rooms know what's connected to them
      (else
        (Variables|Default|SetLoadingLevelsLoopCount (+ (Variables|Default|GetLoadingLevelsLoopCount) 1)) ; Increment our loop count and spawn the next room
        (goto _label)))))

(event Custom|AlignEntranceToExit
  (params (AnchorLocation :type Transform))
  ;[1 1 1] Align the Entrace of this room to the Exit of the previous room
  (if (!= (Variables|Default|GetEntranceAnchorRootObject) 0) ; Do we have an entrance?
    (if (not (Variables|Default|GetHasAlignedEntraceToExit)) ; Have we already aligned this room?
      (bind _returnvalue (Transformation|SetActorTransform (Variables|Default|GetEntranceAnchorRootObject) AnchorLocation)) ; Align this room to the exit from the connecting room
      (Variables|Default|SetHasAlignedEntraceToExit _returnvalue) ; Make sure we don't do this again
    )))

(event Custom|PassConnectedRoomsToNewRooms
  ;[1 1 1] Pass the Connected Room,  The room name, and this room to the newly spawned rooms
  (for _array_element (Variables|Default|GetConnectedRooms)
    (Class|RoomInterfaces|PassConnectedRooms(Message) (Class|GameplayStatics|GetStreamingLevel _array_element) (Variables|Default|GetConnectedRooms) _array_element (Variables|Default|GetCurrentRoom))))

(event Custom|SetRoomsCameFrom
  (params (Rooms :type Array%20of%20Names) (CurrentRoom :type Name) (PreviousRoom :type Name))
  ;[1 1 1] Set our Rooms Variables
  (bind _output_get (Variables|Default|SetRoomsCameFrom Rooms)) ; Which rooms are loaded behind us
  (Variables|Default|SetCurrentRoom CurrentRoom) ; Which room is this
  (Utilities|Array|Add _output_get PreviousRoom) ; Add the prior room to our rooms we came from
)

(fn ConstructionScript)

(fn WhichRoomtoSpawn
  (return (Utilities|Array|Get(acopy) (Variables|Default|GetSpawnableRooms) (Variables|Default|GetLoadingLevelsLoopCount))))