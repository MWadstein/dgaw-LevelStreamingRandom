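; Door Blueprint that slides its mesh by a set offset, once it has finished a full move.
; Overlapping the collision with an actor implementing PlayerInterface calls the AnimateDoor event if IsOpenDoor is set.
; AnimateDoor captures the mesh's world location and uses a timeline to lerp it to the offset position.
; HasTriggered is set only when the timeline finishes, so calls during movement restart it from the current location.
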(event OnComponentBeginOverlap(Collision)
  (params (OtherActor :type Actor%20Object%20Reference) (OtherComp :type Primitive%20Component%20Object%20Reference) (OtherBodyIndex :type Integer) (bFromSweep :type Boolean) (SweepResult :type Hit%20Result%20Structure%20%28by%20ref%29))
  (if (Utilities|DoesObjectImplementInterface OtherActor "/Game/Blueprints/Interfaces/PlayerInterface.PlayerInterface_C")
    (if (Variables|Default|GetIsOpenDoor)
      (CallFunction|AnimateDoor))))

(event Custom|AnimateDoor
  (if (not (Variables|Default|GetHasTriggered))
    (Variables|Default|SetDoorStartingLoc (Transformation|GetWorldLocation (Variables|Default|GetDoorMesh)))
    (Variables|Default|SetDoorEndingLoc (+ (Variables|Default|GetDoorStartingLoc) (Variables|Default|GetDoorEndingOffset)))
    (bind _lerp_0___1 (Timeline|Timeline_0 PlayFromStart)
      (:Update
        (Transformation|SetWorldLocation (Variables|Default|GetDoorMesh) (Math|Vector|Lerp(Vector) (Variables|Default|GetDoorStartingLoc) (Variables|Default|GetDoorEndingLoc) _lerp_0___1) false false))
      (:Finished
        (Variables|Default|SetHasTriggered true)))))

(fn ConstructionScript)